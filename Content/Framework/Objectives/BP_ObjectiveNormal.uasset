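; BP_ObjectiveNormal is a chained objective trigger that advances the player's current normal objective when overlapped.
; On overlap it hands BP_Player the next objective and its objective text, updates the nav point unless final, then destroys itself.
; Every tick it shows itself with collision only while it is the player's current objective.
; Each non-final objective also writes its successor's location to the player's nav point at BeginPlay.
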(event EventBeginPlay
  (if (not (Variables|Objective|GetIsFinalObjective?))
    (bind _asbp_player (Utilities|Casting|CastToBP_Player (Game|Player|GetPlayerPawn 0)))
    (Variables|/Game/Player/BP_Player.BP_Player_C|SetNormalNavPoint _asbp_player (Transformation|GetActorLocation (Variables|Objective|GetNext%20Objective)))
    (Variables|Objective|SetIsNextObjective? false)))

(event Collision|EventActorBeginOverlap
  (params (OtherActor :type Actor%20Object%20Reference))
  (bind _next_objective (Variables|Objective|GetNext%20Objective))
  (bind _asbp_player (Utilities|Casting|CastToBP_Player OtherActor))
  (if (Variables|Objective|GetIsFinalObjective?)
    _
    (else
      (Variables|/Game/Player/BP_Player.BP_Player_C|SetNormalNavPoint _asbp_player (Transformation|GetActorLocation _next_objective))))
  (Variables|/Game/Player/BP_Player.BP_Player_C|SetCurrentNormalObjective _asbp_player _next_objective)
  (Variables|/Game/Player/BP_Player.BP_Player_C|SetCurrentObjectiveText _asbp_player (Variables|Objective|GetObjectiveText))
  (Actor|DestroyActor))

(event EventTick
  (params (DeltaSeconds :type Float%20%28single-precision%29))
  (|ShouldHide?))

(fn ConstructionScript)