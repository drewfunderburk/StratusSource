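; BP_ObjectiveSecure is a capture-point objective that fills while overlapped and destroys itself when secured.
; A timeline plays on overlap and reverses on exit, driving the capture sphere's dynamic material.
; It points the player's secure nav point at itself or NextObjective, and advances the current objective during capture.
; Tick toggles visibility and collision by comparison with the player's current objective; counter-based securing functions are never called.
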(event Collision|EventActorEndOverlap
  (params (OtherActor :type Actor%20Object%20Reference))
  (bind _nextobjective (Variables|Objective|GetNextObjective))
  (bind _value (Timeline|SecureTimeline Reverse)
    (:Update
      (if (>= _value 1.0)
        (Actor|DestroyActor))
      (Rendering|Material|SetScalarParameterValue (Variables|Objective|GetCaptureStatus) "CaptureStatus" _value :!class /Script/Engine.MaterialInstanceDynamic)
      (bind _asbp_player (Utilities|Casting|CastToBP_Player (stale Collision|EventActorBeginOverlap OtherActor)))
      (if (not (Variables|Objective|GetIsOnlyObjective?))
        (if (not (Variables|Objective|GetIsFinalObjective?))
          (Variables|/Game/Player/BP_Player.BP_Player_C|SetSecureNavPoint _asbp_player (Transformation|GetActorLocation _nextobjective))
          (Variables|/Game/Player/BP_Player.BP_Player_C|SetCurrentSecureObjective _asbp_player _nextobjective))))))

(event EventBeginPlay
  (bind _returnvalue (Game|Player|GetPlayerPawn 0))
  (bind _returnvalue_2 (Rendering|Material|CreateDynamicMaterialInstance (Variables|Default|GetSM_VFXSphere_CapturePoint) 0 0 "None" :!class /Script/Engine.PrimitiveComponent))
  (Variables|Objective|SetCaptureStatus _returnvalue_2)
  (if (Variables|Objective|GetIsOnlyObjective?)
    (bind _asbp_player (Utilities|Casting|CastToBP_Player _returnvalue :!label _label))
    (Variables|/Game/Player/BP_Player.BP_Player_C|SetSecureNavPoint _asbp_player (Transformation|GetActorLocation self))
    (elif (Variables|Objective|GetIsFinalObjective?)
      (goto _label)
      (else
        (bind _asbp_player_2 (Utilities|Casting|CastToBP_Player _returnvalue))
        (Variables|/Game/Player/BP_Player.BP_Player_C|SetSecureNavPoint _asbp_player_2 (Transformation|GetActorLocation (Variables|Objective|GetNextObjective)))
        (Variables|Objective|SetIsNextObjective? false)))))

(event Collision|EventActorBeginOverlap
  (params (OtherActor :type Actor%20Object%20Reference))
  (bind _nextobjective (Variables|Objective|GetNextObjective))
  (bind _value (Timeline|SecureTimeline Play)
    (:Update
      (if (>= _value 1.0)
        (Actor|DestroyActor))
      (Rendering|Material|SetScalarParameterValue (Variables|Objective|GetCaptureStatus) "CaptureStatus" _value :!class /Script/Engine.MaterialInstanceDynamic)
      (bind _asbp_player (Utilities|Casting|CastToBP_Player OtherActor))
      (if (not (Variables|Objective|GetIsOnlyObjective?))
        (if (not (Variables|Objective|GetIsFinalObjective?))
          (Variables|/Game/Player/BP_Player.BP_Player_C|SetSecureNavPoint _asbp_player (Transformation|GetActorLocation _nextobjective))
          (Variables|/Game/Player/BP_Player.BP_Player_C|SetCurrentSecureObjective _asbp_player _nextobjective))))))

(event EventTick
  (params (DeltaSeconds :type Float%20%28single-precision%29))
  (|ShouldHide?))

(fn ConstructionScript)