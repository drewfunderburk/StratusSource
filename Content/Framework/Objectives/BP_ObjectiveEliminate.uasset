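; BP_ObjectiveEliminate is an eliminate-objective actor that marks a target enemy and feeds its location to the player's EliminateNavPoint.
; On BeginPlay, a non-final objective points that nav point at NextObjective and clears IsNextObjective.
; Each Tick it snaps its root to the enemy's location and rotation and updates the nav point.
; It clears the reference when the enemy's health runs out, then destroys itself.
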(event EventBeginPlay
  (if (not (Variables|Default|GetIsFinalObjective?))
    (bind _asbp_player (Utilities|Casting|CastToBP_Player (Game|Player|GetPlayerPawn 0)))
    (Variables|/Game/Player/BP_Player.BP_Player_C|SetEliminateNavPoint _asbp_player (Transformation|GetActorLocation (Variables|Default|GetNextObjective)))
    (Variables|Default|SetIsNextObjective? false)))

(event EventTick
  (params (DeltaSeconds :type Float%20%28single-precision%29))
  (bind _enemyreference (Variables|Default|GetEnemyReference))
  (|RemoveReference)
  (Transformation|SetWorldTransform)
  (if (Utilities|IsValid _enemyreference)
    (if (== _enemyreference 0)
      (Actor|DestroyActor)
      (else
        (|ShouldHide?)))
    (else
      (Actor|DestroyActor))))

(fn ConstructionScript)