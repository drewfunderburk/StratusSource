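; BP_EnemyManager tracks the enemies in a level and shows the victory screen when all of them are defeated.
; On BeginPlay it gathers every BP_EnemyBase actor, binds to each one's death event and creates an enemy counter widget.
; Each death removes that enemy from the list and updates the counter.
; At zero, it shows a "Victory" end screen with UI-only input and a visible cursor.
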(event Custom|OnEnemyDeath
  (params (Enemy :type BP%20Enemy%20Base%20Object%20Reference))
  (bind _returnvalue (CallFunction|GetActiveEnemyCount))
  (Utilities|Array|RemoveItem (Variables|Default|GetEnemies) Enemy)
  (Variables|/Game/UI/Widget_EnemyCounter.Widget_EnemyCounter_C|SetEnemyCount (Variables|Default|GetEnemyCounter) _returnvalue)
  (if (== _returnvalue 0)
    (CallFunction|OnAllEnemiesDefeated)))

(event Custom|OnAllEnemiesDefeated
  (bind _returnvalue (Game|GetPlayerController 0))
  ;[1 1 1] Show victory screen
  (bind _returnvalue_2 (UserInterface|CreateWidget "/Game/UI/Widget_EndScreen.Widget_EndScreen_C"))
  (UserInterface|Viewport|AddtoViewport _returnvalue_2 0)
  (Input|SetInputModeUIOnly _returnvalue 0 "DoNotLock")
  (Variables|/Script/Engine.PlayerController|SetbShowMouseCursor _returnvalue true))

(event EventBeginPlay
  (CallFunction|GatherEnemiesinLevel (delegate Custom|OnEnemyDeath))
  (bind _returnvalue (UserInterface|CreateWidget "/Game/UI/Widget_EnemyCounter.Widget_EnemyCounter_C"))
  (bind _output_get (Variables|Default|SetEnemyCounter _returnvalue))
  (UserInterface|Viewport|AddtoViewport _output_get 0)
  (Variables|/Game/UI/Widget_EnemyCounter.Widget_EnemyCounter_C|SetEnemyCount _returnvalue (CallFunction|GetActiveEnemyCount)))

(fn ConstructionScript)

(fn GatherEnemiesinLevel
  (params (Event :type Delegate%20%28by%20ref%29))
  (bind _outactors (Actor|GetAllActorsOfClass "/Game/Enemies/BP_EnemyBase.BP_EnemyBase_C"))
  (bind _output_get (Variables|Default|SetEnemies _outactors))
  (for _array_element _output_get
    (EventDispatchers|BindEventtoOnDeath _array_element Event)))

(fn GetActiveEnemyCount
  (return (Utilities|Array|Length (Variables|Default|GetEnemies))))