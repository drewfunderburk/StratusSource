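; Base enemy airship that fights with broadside cannons and yields a random amount of gold when killed.
; Each tick it pushes ranges, agro state and player location to its AI blackboard and turns its health bar toward the player camera.
; Tag-sorted left and right cannons fire in shuffled, staggered volleys with per-side cooldowns.
; At zero health it awards gold, unpossesses, drops spinning under gravity, then is destroyed after a delay.
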(event Custom|Fire
  (params (Is%20Right%20Side :type Boolean))
  (if Is%20Right%20Side
    (|FireRightSide)
    (else
      (|FireLeftSide))))

(event EventOnTakeDamage
  (params (damage :type Float%20%28single-precision%29) (source :type Actor%20Object%20Reference))
  (bind _healthbar (Variables|Default|GetHealthBar))
  (bind _static_mesh (Variables|Default|GetStatic%20Mesh))
  (bind _returnvalue (Class|EnemyBase|TakeDamage damage))
  (Utilities|IsValid _healthbar
    (:Is%20Valid
      (Variables|/Game/UI/Widget_HealthBar.Widget_HealthBar_C|SetHealth _healthbar (Math|Float|Round _returnvalue)))
    (:Is%20Not%20Valid
      _))
  (if (== _returnvalue 0.0)
    (Default|CallOnDeath self)
    (bind _asstratus_game_instance (Utilities|Casting|CastToStratusGameInstance (Game|GetGameInstance)))
    (Default|AddGold _asstratus_game_instance self)
    (|IsValidUnPossess)
    (|AirshipMovementValidDelete)
    (Class|WidgetComponent|SetTintColorandOpacity (Variables|Default|GetHealth%20Bar) "(R=0.000000,G=0.000000,B=0.000000,A=0.000000)")
    (|IsValidDestroyBillboard)
    (Physics|SetEnableGravity _static_mesh true)
    (Class|PrimitiveComponent|SetAngularDamping _static_mesh 0.1)
    (Class|PrimitiveComponent|AddAngularImpulseinDegrees _static_mesh (Math|Vector|MakeVector (Math|Random|RandomFloatinRange 0.0 (Variables|Default|GetXImpulseScalar)) (Math|Random|RandomFloatinRange 0.0 (Variables|Default|GetYImpulseScalar)) (Math|Random|RandomFloatinRange 0.0 (Variables|Default|GetZImpulseScalar))) "None" true)
    (Utilities|FlowControl|Delay 2e+01)
    (Actor|DestroyActor)))

(event EventTick
  (params (DeltaSeconds :type Float%20%28single-precision%29))
  (CallFunction|DebugDrawAgroRange false)
  (|UpdateBlackboardValues)
  (CallFunction|FaceHealthBartoPlayer))

(event EventBeginPlay
  (Variables|/Game/Player/AC_AirshipMovement.AC_AirshipMovement_C|SetStaticMesh (Variables|Default|GetAC_AirshipMovement) (Variables|Default|GetStatic%20Mesh))
  (|AddCannonstoArrays)
  (|SetUpHealthBar)
  (|GetPlayer)
  (|SetGoldYield))

(fn ConstructionScript)

(fn DebugDrawAgroRange
  (params (Draw? :type Boolean))
  (bind _returnvalue (Transformation|GetActorLocation))
  (if Draw?
    (Rendering|Debug|DrawDebugSphere _returnvalue (Variables|AI|GetAgro%20Range) 12 "(R=1.000000,G=0.000000,B=0.000000,A=1.000000)" 0.0)
    (Rendering|Debug|DrawDebugSphere _returnvalue (Variables|AI|GetDeAgro%20Range) 12 "(R=0.000000,G=1.000000,B=0.000000,A=1.000000)" 0.0)
    (Rendering|Debug|DrawDebugSphere _returnvalue (Variables|AI|GetBroadside%20Range) 12 "(R=0.000000,G=0.000000,B=1.000000,A=1.000000)" 0.0)))

(fn FaceHealthBartoPlayer
  (bind _health_bar (Variables|Default|GetHealth%20Bar))
  (Utilities|IsValid _health_bar
    (:Is%20Valid
      (Transformation|SetWorldRotation _health_bar (Math|Rotator|FindLookatRotation (Transformation|GetWorldLocation _health_bar) (Transformation|GetWorldLocation (Variables|/Game/Player/BP_Player.BP_Player_C|GetCamera (Variables|Default|GetPlayer)))) false false))
    (:Is%20Not%20Valid)))