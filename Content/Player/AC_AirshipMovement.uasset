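; Airship movement component that flies its owner by applying physics forces and torques to a static mesh.
; Each tick it applies forward thrust from a stepped speed level, adds roll from current roll and sideways velocity, and corrects pitch beyond a limit.
; Pitch, yaw and roll helpers build torque with TransformLocation, which includes world position.
; AddTorqueTowardsRotation steers toward a target using clamped yaw and pitch deltas.
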(event EventTick
  (params (DeltaSeconds :type Float%20%28single-precision%29))
  (bind _returnvalue (Components|GetOwner))
  (bind _staticmesh (Variables|Default|GetStaticMesh))
  (bind _returnvalue_2 (Transformation|GetWorldRotation _staticmesh))
  ;[1 1 1] Thrust
  (Physics|AddForce (Variables|Default|GetStaticMesh) (* (* (Math|Vector|GetForwardVector (Variables|Default|GetStaticMesh)) (Utilities|Array|Get(acopy) (Variables|Default|GetSpeedLevels) (Variables|Default|GetSpeedLevel))) (Variables|Default|GetThrustForce)) "None" false)
  ;[1 1 1] Roll compensation
  (CallFunction|AddRoll (Math|Float|MapRangeClamped (.roll (Transformation|GetWorldRotation (Variables|Default|GetStaticMesh))) -45.0 45.0 -1.0 1.0) false)
  ;[1 1 1] Rol with Velocity
  (CallFunction|AddRoll (* (.y (Math|Vector|UnrotateVector (Math|Vector|Normalize (Transformation|GetVelocity _returnvalue)) (Transformation|GetActorRotation _returnvalue))) -1.0) false)
  ;[1 1 1] Pitch clamping
  (if (> (.pitch _returnvalue_2) (Variables|Default|GetMaximumPitchAngle))
    (CallFunction|AddPitch (Math|Float|MapRangeClamped (.pitch _returnvalue_2) (Variables|Default|GetMaximumPitchAngle) (Variables|Default|GetMaximumOverpitchAngle) 0.0 2.0))
    (elif (< (.pitch _returnvalue_2) (* (Variables|Default|GetMaximumPitchAngle) -1.0))
      (CallFunction|AddPitch (Math|Float|MapRangeClamped (.pitch _returnvalue_2) (* (Variables|Default|GetMaximumPitchAngle) -1.0) (* (Variables|Default|GetMaximumOverpitchAngle) -1.0) 0.0 -2.0)))))

(fn IncreaseThrust
  (if (< (+ (Variables|Default|GetSpeedLevel) 1) (Utilities|Array|Length (Variables|Default|GetSpeedLevels)))
    (Variables|Default|SetSpeedLevel (+ (Variables|Default|GetSpeedLevel) 1))))

(fn DecreaseThrust
  (if (> (- (Variables|Default|GetSpeedLevel) 1) -1)
    (Variables|Default|SetSpeedLevel (- (Variables|Default|GetSpeedLevel) 1))))

(fn AddPitch
  (params (Value :type Float%20%28single-precision%29))
  (bind _staticmesh (Variables|Default|GetStaticMesh))
  (Utilities|IsValid _staticmesh
    (:Is%20Valid
      (Class|PrimitiveComponent|AddTorqueinRadians _staticmesh (Math|Transform|TransformLocation (Transformation|GetWorldTransform _staticmesh) (Math|Vector|MakeVector 0.0 (* Value (Variables|Default|GetPitchForce)) 0.0)) "None" false))
    (:Is%20Not%20Valid
      (Development|PrintString "Static Mesh is not valid" true true "(R=1.000000,G=0.000000,B=0.000000,A=1.000000)"))))

(fn AddYaw
  (params (Value :type Float%20%28single-precision%29))
  (bind _staticmesh (Variables|Default|GetStaticMesh))
  (Utilities|IsValid _staticmesh
    (:Is%20Valid
      (Class|PrimitiveComponent|AddTorqueinRadians _staticmesh (Math|Transform|TransformLocation (Transformation|GetWorldTransform _staticmesh) (Math|Vector|MakeVector 0.0 0.0 (* Value (Variables|Default|GetYawForce)))) "None" false))
    (:Is%20Not%20Valid
      (Development|PrintString "Static Mesh is not valid" true true "(R=1.000000,G=0.000000,B=0.000000,A=1.000000)"))))

(fn AddRoll
  (params (Value :type Float%20%28single-precision%29) (Impulse? :type Boolean))
  (bind _staticmesh (Variables|Default|GetStaticMesh))
  (bind _rollforce (Variables|Default|GetRollForce))
  (bind _returnvalue (Transformation|GetWorldTransform _staticmesh))
  (bind _returnvalue_2 (* Value _rollforce))
  (bind _returnvalue_3 (Math|Transform|TransformLocation _returnvalue (Math|Vector|MakeVector _returnvalue_2 0.0 0.0)))
  (Utilities|IsValid _staticmesh
    (:Is%20Valid
      (if Impulse?
        (Class|PrimitiveComponent|AddAngularImpulseinRadians _staticmesh _returnvalue_3 "None" false)
        (else
          (Class|PrimitiveComponent|AddTorqueinRadians _staticmesh _returnvalue_3 "None" false))))
    (:Is%20Not%20Valid
      (Development|PrintString "Static Mesh is not valid" true true "(R=1.000000,G=0.000000,B=0.000000,A=1.000000)"))))

(fn AddTorqueTowardsRotation
  (params (Rotation :type Rotator))
  (bind _returnvalue (Components|GetOwner))
  (bind _returnvalue_2 (Transformation|GetActorRotation _returnvalue))
  (bind _returnvalue_3 (Math|Rotator|Delta(Rotator) Rotation _returnvalue_2))
  (CallFunction|AddYaw (Math|Float|Clamp(Float) (.yaw _returnvalue_3) -1.0))
  (CallFunction|AddPitch (Math|Float|Clamp(Float) (.pitch _returnvalue_3) -1.0)))