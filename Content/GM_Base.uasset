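; Base game mode that manages a single save slot using BP_SaveGame.
; On BeginPlay it checks for "Save1", then either loads the slot named by SlotName or creates and writes a fresh save there.
; SaveGame reloads "Save1" and writes it back to SlotName without changing any data.
; LoadGame only restarts the level via console command, while RestartLevel deletes the SlotName save first.
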(event Custom|SaveGame
  (bind _returnvalue (SaveGame|LoadGamefromSlot "Save1"))
  (bind _asbp_save_game (Utilities|Casting|CastToBP_SaveGame _returnvalue))
  (SaveGame|SaveGametoSlot _asbp_save_game (Variables|Default|GetSlot%20Name)))

(event Custom|LoadGame
  ;[1 1 1] Load Game
  (Development|ExecuteConsoleCommand "RestartLevel" 0))

(event Custom|RestartLevel
  ;[1 1 1] Delete and Restart level
  (SaveGame|DeleteGameinSlot (Variables|Default|GetSlot%20Name))
  (Development|ExecuteConsoleCommand "RestartLevel" 0))

(event EventBeginPlay
  (bind _returnvalue (SaveGame|DoesSaveGameExist "Save1"))
  (if _returnvalue
    (bind _returnvalue_2 (SaveGame|LoadGamefromSlot (Variables|Default|GetSlot%20Name)))
    (Utilities|Casting|CastToBP_SaveGame _returnvalue_2)
    (else
      ;[1 1 1] Create save file
      (bind _returnvalue_3 (SaveGame|CreateSaveGameObject "/Game/Framework/SaveGame/BP_SaveGame.BP_SaveGame_C"))
      (SaveGame|SaveGametoSlot _returnvalue_3 (Variables|Default|GetSlot%20Name)))))

(fn ConstructionScript)