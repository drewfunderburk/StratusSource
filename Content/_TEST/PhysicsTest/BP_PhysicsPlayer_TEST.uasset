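; BP_PhysicsPlayer_TEST is a test player Blueprint for flying an airship through the ACAirshipMovement component.
; Pitch and Yaw axis inputs feed straight into the component, and the throttle actions increase or decrease thrust on each press.
; On BeginPlay it passes its StaticMesh to the component, which handles all movement logic outside this graph.
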(event EventBeginPlay
  (Variables|/Game/Player/AC_AirshipMovement.AC_AirshipMovement_C|SetStaticMesh (Variables|Default|GetAC_AirshipMovement) (Variables|Default|GetStatic%20Mesh)))

(event Input|ActionEvents|InputActionIncreaseThrottle
  (params (Key :type Key%20Structure))
  ;[1 1 1] Throttle
  (:Pressed
    (Default|IncreaseThrust (Variables|Default|GetAC_AirshipMovement))))

(event Input|ActionEvents|InputActionDecreaseThrottle
  (params (Key :type Key%20Structure))
  ;[1 1 1] Throttle
  (:Pressed
    (Default|DecreaseThrust (Variables|Default|GetAC_AirshipMovement))))

(event Input|AxisEvents|InputAxisPitch
  (params (AxisValue :type Float%20%28single-precision%29))
  ;[1 1 1] Rotation Controls
  (Default|AddPitch (Variables|Default|GetAC_AirshipMovement) AxisValue))

(event Input|AxisEvents|InputAxisYaw
  (params (AxisValue :type Float%20%28single-precision%29))
  ;[1 1 1] Rotation Controls
  (Default|AddYaw (Variables|Default|GetAC_AirshipMovement) AxisValue))

(fn ConstructionScript)