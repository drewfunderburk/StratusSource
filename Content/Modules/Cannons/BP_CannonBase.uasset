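; Base cannon actor that fires projectiles after a delay, with pitch-varied sound, a Niagara effect and a smoke emitter.
; OnFire waits, broadcasts OnFired and spawns the projectile at SpawnTransform with random accuracy offsets, speed, range and player pawn velocity.
; Tick tracks per-frame cannon displacement for the velocity-based aim rotation.
; Tick also calls ClampFireAngle, whose limits center on the current rotation, so it never constrains it.
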(event EventOnFire
  (params (delay :type Float%20%28single-precision%29))
  (Utilities|FlowControl|Delay delay)
  (Default|CallOnFired)
  (CallFunction|Fire (Variables|Default|GetProjectile))
  (Utilities|FlowControl|Delay 0.4)
  (Components|Activation|Deactivate (Variables|Default|GetNP_CannonFX)))

(event EventTick
  (params (DeltaSeconds :type Float%20%28single-precision%29))
  (bind _returnvalue (Transformation|GetActorLocation))
  (|ClampFireAngle)
  (Variables|Default|SetCannonVelocity (- _returnvalue (Variables|Default|GetPositionLastFrame)))
  (Variables|Default|SetPositionLastFrame _returnvalue))

(fn ConstructionScript)

(fn Fire
  (params (Projectile :type BP%20Projectile%20Base%20Class%20Reference))
  (bind _returnvalue (|GetVelocityRotation))
  (bind _spawn_transform (Variables|Default|GetSpawn%20Transform))
  (bind _sfx_singlecannon (Variables|Default|GetSFX_SingleCannon))
  (bind _returnvalue_2 (Transformation|GetWorldTransform _spawn_transform))
  (Audio|Components|Audio|SetPitchMultiplier _sfx_singlecannon (Math|Float|Lerp 0.75 1.25 (Math|Random|RandomFloat)))
  (Audio|Components|Audio|Play _sfx_singlecannon 0.0)
  (Components|Activation|Activate (Variables|Default|GetNP_CannonFX) false)
  (Effects|SpawnEmitteratLocation "/Game/FX/Particles/P_Smoke.P_Smoke" (.location _returnvalue_2) (.rotation _returnvalue_2))
  (Game|SpawnActorfromClass Projectile (Math|Transform|MakeTransform (Transformation|GetWorldLocation (Variables|Default|GetSpawn%20Transform)) (Math|Rotator|MakeRotator (.roll _returnvalue) (+ (.pitch _returnvalue) (Math|Random|RandomFloatinRange (* (Variables|Default|GetverticalAccuracyOffset) -1.0) 0.0)) (+ (.yaw _returnvalue) (Math|Random|RandomFloatinRange (* (Variables|Default|GethorizontalAccuracyOffset) -1.0) 0.0)))) "Undefined" 0 (Variables|Default|GetprojectileSpeed) (Variables|Default|Getrange) (Transformation|GetVelocity (Game|Player|GetPlayerPawn 0)) 0))