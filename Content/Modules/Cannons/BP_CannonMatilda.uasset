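; Cannon Blueprint for the Matilda module, which fires a BP_ProjectileMatilda whenever its Fire event runs.
; MatildaFire activates the cannon's FX component and spawns a smoke emitter at the SpawnTransform component.
; It then spawns the scaled-up projectile there, randomising pitch and yaw with the vertical and horizontal accuracy offsets and passing in projectile speed and range.
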(event EventFire
  (params (Projectile :type BP%20Projectile%20Base%20Class%20Reference))
  (|MatildaFire))

(fn ConstructionScript
  (|CallParentFunction))