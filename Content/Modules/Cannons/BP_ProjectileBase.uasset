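; Base projectile for the cannons module that damages what it hits and expires based on its range.
; Construction applies MaxSpeed to ProjectileMovement and derives lifespan from MaxRange / MaxSpeed.
; BeginPlay adds the X component of InheritedVelocity to the movement's InitialSpeed.
; Any sphere overlap destroys it, first sending OnTakeDamageMessage if the other actor implements the Damageable interface.
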(event OnComponentBeginOverlap(SphereCollision)
  (params (OverlappedComponent :type Primitive%20Component%20Object%20Reference) (OtherActor :type Actor%20Object%20Reference) (OtherComp :type Primitive%20Component%20Object%20Reference) (OtherBodyIndex :type Integer) (bFromSweep :type Boolean) (SweepResult :type Hit%20Result%20Structure%20%28by%20ref%29))
  (if (Utilities|DoesObjectImplementInterface OtherActor "/Script/Stratus.Damageable")
    (Class|Damageable|OnTakeDamage(Message) OtherActor (Variables|Default|GetDamage) self))
  (Actor|DestroyActor))

(event EventBeginPlay
  (bind _projectilemovement (Variables|Default|GetProjectileMovement))
  (Variables|/Script/Engine.ProjectileMovementComponent|SetInitialSpeed _projectilemovement (+ (.x (Variables|Default|GetInheritedVelocity)) (Variables|/Script/Engine.ProjectileMovementComponent|GetInitialSpeed _projectilemovement))))

(fn ConstructionScript
  (bind _max_speed (Variables|Default|GetMax%20Speed))
  (bind _projectilemovement (Variables|Default|GetProjectileMovement))
  (Utilities|FlowControl|Sequence
    (:then_0
      (CallFunction|SetProjectileSettings _max_speed (Variables|Default|GetMax%20Range)))
    (:then_1
      (Variables|/Script/Engine.ProjectileMovementComponent|SetInitialSpeed _projectilemovement _max_speed))
    (:then_2
      (Variables|/Script/Engine.ProjectileMovementComponent|SetMaxSpeed _projectilemovement _max_speed))))

(fn SetProjectileSettings
  (params (Max%20Speed :type Float%20%28single-precision%29) (Max%20Range :type Float%20%28single-precision%29))
  (bind _output_get (Variables|Default|SetMax%20Speed Max%20Speed))
  (bind _output_get_2 (Variables|Default|SetMax%20Range Max%20Range))
  (Actor|SetLifeSpan (/ _output_get_2 _output_get)))